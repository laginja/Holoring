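; Capturable flag actor that a FirstPersonCharacter picks up by overlapping it.
; On overlap it stores the player and, if that player is not already holding a flag, snaps to their FlagSocket and sets their IsHoldingFlag.
; Server events forward to Multi events that detach the flag or detach and destroy it, each printing a debug message.
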(event `self.ReceiveActorBeginOverlap`
  (params (OtherActor :type "Actor Object Reference"))
  (bind _asfirst_person_character (cast `/Game/Character/FirstPersonCharacter` OtherActor))
  (`/Engine/EditorBlueprintResources/StandardMacros.IsValid` _asfirst_person_character
    (:`Is Valid`
      (bind _output_get (set `self.Player` _asfirst_person_character))
      (if (not (`/Game/Character/FirstPersonCharacter.bIsHoldingFlag` (`self.Player`)))
        (`self.K2_AttachToActor` _output_get "FlagSocket" "SnapToTarget" "SnapToTarget" "KeepWorld" false)
        (set `/Game/Character/FirstPersonCharacter.bIsHoldingFlag` true _asfirst_person_character)))))

(event `ServerDestroyFlag`
  (`self.MultiDestroyFlag`))

(event `MultiDestroyFlag`
  (`self.K2_DetachFromActor` "KeepWorld" "KeepWorld" "KeepWorld")
  (`self.K2_DestroyActor`)
  (`KismetSystemLibrary.PrintString` "Hello DESTROYED"))

(event `ServerDetachFlag`
  (`self.MultiDetachFlag`))

(event `MultiDetachFlag`
  (`self.K2_DetachFromActor` "KeepWorld" "KeepWorld" "KeepWorld")
  (`KismetSystemLibrary.PrintString` "Hello DETACHEEEEEEED"))

(fn `UserConstructionScript`)