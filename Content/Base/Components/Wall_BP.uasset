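; Wall actor that starts hidden without collision and becomes a solid, visible wall when built.
; BeginPlay hides the static mesh component and disables its collision.
; The BuildAWall event relays through a CL-prefixed build event to CreateWall, which shows the mesh and enables query and physics collision.
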(event `self.ReceiveBeginPlay`
  (`SceneComponent.SetVisibility` (`self.StaticMeshComponent`) false false)
  (`PrimitiveComponent.SetCollisionEnabled` (`self.StaticMeshComponent`) "NoCollision"))

(event `BuildAWall`
  (`self.CL_BuildAWall`))

(event `CL_BuildAWall`
  (`self.CreateWall`))

(fn `CreateWall`
  (`SceneComponent.SetVisibility` (`self.StaticMeshComponent`) true false)
  (`PrimitiveComponent.SetCollisionEnabled` (`self.StaticMeshComponent`) "QueryAndPhysics"))

(fn `UserConstructionScript`)