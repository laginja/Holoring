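; Chest actor that demonstrates replication approaches, toggling its lid open and closed according to a selected ReplicationType.
; ToggleOpen picks a local event, a multicast adding one-time sound and particles, a RepNotify that snaps the lid, or multicast followed by RepNotify once opening finishes.
; A timeline drives lid rotation with ForceNetUpdate, then updates emissive strength.
; The construction script sets up the dynamic material and a sphere visualizing net cull distance.
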(event `NR_ToggleOpen`
  ;[0 0 0 0.25] Part 4 - Multicast & RepNotify
  ;;[0 1 0 0.25] Not Replicated
  (bind _isa (`/Engine/EditorBlueprintResources/StandardMacros.FlipFlop` :!label _label)
    (:`A`
      (bind (_direction _alpha) (`Timeline|OpenChest` :!via `PlayFromStart` :!label _label_2)
        (:`Update`
          (`self.Open` _alpha))
        (:`Finished`
          (`self.UpdateEmissive` _isa)
          ;;[1 0 0 0.25] If Multicast & Repnotify, call the RepNotify when the chest has finished opening
          (if (`|EnumEquality` (`self.ReplicationType`) "NewEnumerator3")
            (`self.RN_ToggleOpen`)))))
    (:`B`
      (goto _label_2 :!via `ReverseFromEnd`))))

(event `MC_ToggleOpen`
  (bind _returnvalue (`self.K2_GetActorLocation`))
  ;[0 0 0 0.25] Part 4 - Multicast & RepNotify
  ;;[0 0.4 1 0.25] Multicast
  (`GameplayStatics.PlaySoundAtLocation` "/Game/YouTube/Assets/3rdParty/Sounds/ChestOpen.ChestOpen" _returnvalue (struct) 1.0 1.0 0.0 null null null)
  (`GameplayStatics.SpawnEmitterAtLocation` "/Game/YouTube/Assets/3rdParty/Particles/ParticleSystems/Par_RainBlow_01.Par_RainBlow_01" (`KismetMathLibrary.MakeVector` (.x _returnvalue) (- (.y _returnvalue) 200.0) 10.0) (struct :`Yaw` 90.0) (2.0 2.0 2.0))
  (goto _label))

(event `ToggleOpen`
  ;[0 0 0 0.25] Part 4 - Multicast & RepNotify
  (switch `/Game/YouTube/Replication/Part4-MulticastAndRepnotify/Blueprints/E_Replication` (`self.ReplicationType`)
    (:`NewEnumerator0`
      ;;[0 1 0 0.25] Not Replicated
      (`self.NR_ToggleOpen`))
    (:`NewEnumerator1`
      ;;[0 0.4 1 0.25] Multicast
      (`self.MC_ToggleOpen`))
    (:`NewEnumerator2`
      ;;[1 1 0 0.25] RepNotify
      (`self.RN_ToggleOpen`))
    (:`NewEnumerator3`
      ;;[1 0 0 0.25] Multicast then RepNotify
      (`self.MC_ToggleOpen`))))

(event `RN_ToggleOpen`
  ;[0 0 0 0.25] Part 4 - Multicast & RepNotify
  ;;[1 1 0 0.25] RepNotify
  (set `self.IsOpen?` (not (`self.IsOpen?`))))

(fn `OnRep_IsOpen?`
  (`SceneComponent.K2_SetRelativeRotation` (`self.Top`) (select `bool` (`self.IsOpen?`) :`true` (struct :`Pitch` 130.0) :!type "Rotator Structure") false false))

(fn `Open`
  (params (Alpha :type "Float (double-precision)"))
  (`SceneComponent.K2_SetRelativeRotation` (`self.Top`) (`KismetMathLibrary.RLerp` (struct) (struct :`Pitch` 130.0) Alpha) false false)
  (`self.ForceNetUpdate`))

(fn `SetMaterial`
  (locals (Material :type "MaterialInstanceDynamic Object Reference"))
  (bind _returnvalue (`KismetMaterialLibrary.CreateDynamicMaterialInstance` "/Game/YouTube/Assets/Materials/Instances/Chest/MI_Chest.MI_Chest"))
  (bind _output_get (set `self.Materials` _returnvalue))
  (`PrimitiveComponent.SetMaterial` (`self.Top`) 0 _output_get)
  (`PrimitiveComponent.SetMaterial` (`self.Bottom`) 0 _output_get)
  (`MaterialInstanceDynamic.SetVectorParameterValue` _output_get "EmissiveColor" (`self.EmissiveColor`))
  (`MaterialInstanceDynamic.SetScalarParameterValue` _output_get "EmissiveStrength" (`self.EmissiveStrength`)))

(fn `UpdateEmissive`
  (params (InputPin :type Boolean))
  (`MaterialInstanceDynamic.SetScalarParameterValue` (`self.Materials`) "EmissiveStrength" (select `bool` InputPin :`false` (`self.EmissiveStrength`))))

(fn `UserConstructionScript`
  (`SceneComponent.SetWorldScale3D` (`self.Sphere`) (`KismetMathLibrary.Conv_DoubleToVector` (* 2 (`KismetMathLibrary.Sqrt` (`self.NetCullDistanceSquared`)))))
  (`SceneComponent.SetVisibility` (`self.Sphere`) (`self.ShowRelevancyArea?`) false)
  (`self.SetMaterial`))