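; Player controller for the first-person character that creates the local player's UI and handles death and scoring.
; On death it ragdolls the pawn, unpossesses it, then re-possesses the same pawn after a delay.
; The game mode's RespawnPlayer call is left unwired.
; Score increases run on authority, notifying LevelGameModeBase_BP and having HoloringPlayerState_BP print the score.
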(event `self.ReceiveBeginPlay`
  (if (`self.IsLocalPlayerController`)
    (bind _returnvalue (`|CreateWidget` "/Game/Character/UI/WBP_CharacterUI.WBP_CharacterUI_C" self))
    (bind _output_get (set `self.PlayerUI` _returnvalue))
    (`UserWidget.AddToViewport` _output_get 0)))

(event `self.PlayerDied`
  (params (PlayerController :type "FPCharacterPlayerController Object Reference"))
  ;[1 1 1] Event for player death / Respawn player
  (bind _asfirst_person_character (cast `/Game/Character/FirstPersonCharacter` (`self.K2_GetPawn`)))
  (`/Game/Character/FirstPersonCharacter.TurnToRagdoll` _asfirst_person_character)
  (`self.UnPossess`)
  (`KismetSystemLibrary.Delay` 3.0)
  (`self.Possess` _asfirst_person_character)
  (`/Engine/EditorBlueprintResources/ActorMacros.Switch Has Authority`
    (:`Authority`
      (bind _aslevel_game_mode_base_bp (cast `/Game/GameMode/LevelGameModeBase_BP` (`GameplayStatics.GetGameMode`))))))

(event `self.IncreaseScore`
  ;[0.4271 1 0.4927] Increase player score on elimination
  (`/Engine/EditorBlueprintResources/ActorMacros.Switch Has Authority`
    (:`Authority`
      (bind _aslevel_game_mode_base_bp (cast `/Game/GameMode/LevelGameModeBase_BP` (`GameplayStatics.GetGameMode`)))
      (`/Game/GameMode/LevelGameModeBase_BP.PlayerScored` _aslevel_game_mode_base_bp self)
      (bind _asholoring_player_state_bp (cast `/Game/Character/HoloringPlayerState_BP` (`self.PlayerState`)))
      (`/Game/Character/HoloringPlayerState_BP.PrintScore` _asholoring_player_state_bp))))

(fn `UserConstructionScript`)