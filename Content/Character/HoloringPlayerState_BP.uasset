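; Player state Blueprint that holds a player's score, team and class.
; SR_-prefixed events set the team to Alpha or Bravo and store the chosen character class as its display name.
; The score can be printed or read through a getter, but nothing here changes it.
; GetSpawnPoint contains only unconnected random-pick transform nodes, so it is unfinished.
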(event `PrintScore`
  ;[1 1 1] Print player score
  (`KismetSystemLibrary.PrintString` (`KismetStringLibrary.Conv_IntToString` (`self.PlayerScore`))))

(event `SR_SetTeamA`
  ;[1 1 1] Assign player to a team
  (set `self.PlayerTeam` "Alpha"))

(event `SR_SetTeamB`
  ;[1 1 1] Assign player to a team
  (set `self.PlayerTeam` "Bravo"))

(event `SR_SetPlayerClass`
  (params (`Character Class` :type "Character Class Reference"))
  (set `self.PlayerClass` (`KismetSystemLibrary.GetClassDisplayName` `Character Class`)))

(fn `GetPlayerScore`
  (returns (PlayerScore :type Integer))
  (return (`self.PlayerScore`)))

(fn `UserConstructionScript`)